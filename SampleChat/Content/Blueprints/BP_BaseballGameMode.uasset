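; Game mode for a number-baseball guessing game that holds the secret three-digit answer.
; BeginPlay generates and stores the random number, then prints it on screen.
; TurnTimerStart forwards to StartTurnTimer, while GotMessageFromClient is an empty stub.
; A disconnected chain, which never runs, would compare against the answer and broadcast the result to every BP_Controller.
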(event Custom|GotMessageFromClient
  (params (Msg :type Array%20of%20Integers)))

(event Custom|TurnTimerStart
  (Class|BaseballGameMode|StartTurnTimer))

(event EventBeginPlay
  (bind _returnvalue (Class|BaseballGameMode|GenerateRandomThreeDigitNumber))
  (bind _output_get (Variables|Default|SetRandomNumber _returnvalue))
  (Development|PrintString (Utilities|String|ToString(Text) (Utilities|Text|FormatText "{first}{second}{third}" (Utilities|Array|Get(acopy) _output_get) (Utilities|Array|Get(acopy) _output_get 1) (Utilities|Array|Get(acopy) _output_get 2)))))

(event EventTick
  (params (DeltaSeconds :type Float%20%28single-precision%29)))

(fn ConstructionScript)