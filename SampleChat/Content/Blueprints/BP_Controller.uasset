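; BP_Controller links the chat window to the game mode and game state in a networked, chat-driven baseball game.
; After a short BeginPlay delay, it binds to the chat widget's message event and the game state's time and turn updates.
; Login stores the user ID on the player state and starts the turn timer.
; Sent messages become arrays for the game mode, while broadcasts are relayed and printed as results.
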(event Custom|OnSendMsgToServer
  (params (Msg :type String))
  (bind _returnvalue (Class|MyBlueprintFunctionLibrary|ConvertStringtoArray Msg))
  (bind _asbp_baseball_game_mode (Utilities|Casting|CastToBP_BaseballGameMode (Game|GetGameMode)))
  (Default|GotMessagefromClient _asbp_baseball_game_mode _returnvalue))

(event Custom|OnLoginWithID
  (params (UserId :type String))
  (Default|CallOnUserLogin UserId)
  (Utilities|FlowControl|Delay 1.0)
  (bind _asbp_baseball_player_state (Utilities|Casting|CastToBP_BaseballPlayerState (Variables|/Script/Engine.Controller|GetPlayerState (Game|GetPlayerController 0)))
    (:then
      (Class|BaseballPlayerState|SetUserId _asbp_baseball_player_state UserId)
      (bind _asbp_baseball_game_mode (Utilities|Casting|CastToBP_BaseballGameMode (Game|GetGameMode)))
      (Default|TurnTimerStart _asbp_baseball_game_mode))
    (:CastFailed
      (Development|PrintText "Casting Failed"))))

(event Custom|GotBroadcast
  (params (Msg :type String))
  (Default|CallOnPrintResult Msg)
  (Development|PrintString "Hello" true true "(R=0.000000,G=0.660000,B=1.000000,A=1.000000)" 1e+01)
  (Utilities|Casting|CastToBP_BaseballGameState (Game|GetGameState)))

(event EventBeginPlay
  (if (not (Utilities|Enum|Equal(Enum) (Class|Actor|GetRemoteRole) "ROLE_None"))
    (Utilities|FlowControl|Delay 0.5)
    (bind _foundwidgets (Widget|GetAllWidgetsOfClass "/Game/Widgets/Widget_ChatWindow.Widget_ChatWindow_C" true))
    (bind _output_get (Variables|Default|SetWidget (Utilities|Array|Get(acopy) _foundwidgets)))
    (Utilities|FlowControl|Sequence
      (:then_0
        (bind _aswidget_chat_window (Utilities|Casting|CastToWidget_ChatWindow _output_get))
        (EventDispatchers|BindEventtoSetMessagetoUserController _aswidget_chat_window (EventDispatchers|CreateEvent :!event Custom|OnSendMsgToServer)))
      (:then_1
        (bind _asbp_baseball_game_state (Utilities|Casting|CastToBP_BaseballGameState (Game|GetGameState)))
        (EventDispatchers|BindEventtoOnTimeUpdated _asbp_baseball_game_state (EventDispatchers|CreateEvent _aswidget_chat_window :!event UpdateTime)))
      (:then_2
        (EventDispatchers|BindEventtoOnTurnUpdated _asbp_baseball_game_state (EventDispatchers|CreateEvent _aswidget_chat_window :!event UpdateTurn))))))

(fn ConstructionScript)